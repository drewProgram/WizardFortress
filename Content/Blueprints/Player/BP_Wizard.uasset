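; BP_Wizard is the player wizard Blueprint that routes Enhanced Input actions to skill casting, consumable use, interaction and menu closing.
; It delegates to SkillManager, ConsumableManager and the player controller's UI manager, with Skill1 casting Magic Arrow.
; One stored interactable, set and cleared by add/remove events, receives an interface message on interact.
; Any damage becomes a negative health request to AttributeSystem with debug text, while RequestSkill is empty.
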(event `EnhancedInput|/Game/Input/Actions/IA_Skill1`
  (params (ActionValue :type Boolean) (ElapsedSeconds :type "Float (double-precision)") (TriggeredSeconds :type "Float (double-precision)") (InputAction :type "InputAction Object Reference" :default "/Game/Input/Actions/IA_Skill1.IA_Skill1"))
  ; Input handling
  (:`Triggered`
    (`SkillManager.TryCastSkill` (`self.SkillManager`) (struct :`TagName` "Skill.Id.MagicArrow"))))

(event `EnhancedInput|/Game/Input/Actions/IA_UseConsumable`
  (params (ActionValue :type Boolean) (ElapsedSeconds :type "Float (double-precision)") (TriggeredSeconds :type "Float (double-precision)") (InputAction :type "InputAction Object Reference" :default "/Game/Input/Actions/IA_UseConsumable.IA_UseConsumable"))
  ; Input handling
  (:`Triggered`
    (`ConsumableManager.UseActiveConsumable` (`self.ConsumableManager`))))

(event `self.ReceiveBeginPlay`
  (bind _asbp_wfss_player_controller (cast `/Game/Blueprints/Player/BP_WFSS_PlayerController` (`GameplayStatics.GetPlayerController` 0)))
  (set `self.PlayerController` _asbp_wfss_player_controller))

(event `EnhancedInput|/Game/Input/Actions/IA_Interact`
  (params (ActionValue :type Boolean) (ElapsedSeconds :type "Float (double-precision)") (TriggeredSeconds :type "Float (double-precision)") (InputAction :type "InputAction Object Reference" :default "/Game/Input/Actions/IA_Interact.IA_Interact"))
  (bind _interactable (`self.Interactable`))
  ; Input handling
  (:`Triggered`
    (if (`KismetSystemLibrary.IsValid` _interactable)
      (if (`KismetSystemLibrary.DoesImplementInterface` _interactable "/Script/WizardFortress.Interactable")
        (message `Interactable.HandleOnInteracted` _interactable self)
        (set `self.Is Interacting` true)))))

(event `EnhancedInput|/Game/Input/Actions/IA_CloseMenu`
  (params (ActionValue :type Boolean) (ElapsedSeconds :type "Float (double-precision)") (TriggeredSeconds :type "Float (double-precision)") (InputAction :type "InputAction Object Reference" :default "/Game/Input/Actions/IA_CloseMenu.IA_CloseMenu"))
  ; Input handling
  (:`Triggered`
    (`UIManagerComponent.CloseTopScreen` (`WizardFortressPlayerController.GetUIManager` (`self.PlayerController`)))))

(event `self.ReceiveAnyDamage`
  (params (Damage :type "Float (single-precision)") (DamageType :type "DamageType Object Reference") (InstigatedBy :type "Controller Object Reference") (DamageCauser :type "Actor Object Reference"))
  (bind _returnvalue (* Damage -1.0))
  (`AttributeSystem.RequestUpdateHealth` (`self.AttributeSystem`) _returnvalue)
  (`KismetSystemLibrary.PrintText` (`|FormatText` "Should take {damage} damage" _returnvalue)))

(event `self.AddInteractable`
  (params (Interactable :type "Actor Object Reference"))
  (set `self.Interactable` Interactable))

(event `self.RemoveInteractable`
  (set `self.Interactable` null))

(fn `Request Skill`
  (params (Skill :type "GameplayTag Structure") (SpawnLocation :type "Transform Structure")))

(fn `UserConstructionScript`)