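; Interactable storage chest that opens an inventory transfer screen between the interacting actor's inventory and its own.
; InteractArea overlaps add or remove the interaction prompt on actors implementing the Interactor interface.
; Interaction opens the screen through the player controller's UI manager while a timeline rotates the lid, then switches input mapping to UI.
; The manager's last-screen-closed event plays a second lid timeline; item functions are unimplemented stubs.
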(event `self.HandleOnInteracted`
  (params (Instigator :type "BaseCharacter Object Reference"))
  (set `self.ChestOpener` Instigator)
  (bind _asbp_wfss_player_controller (cast `/Game/Blueprints/Player/BP_WFSS_PlayerController` (`GameplayStatics.GetPlayerController` 0)))
  (set `self.PlayerController` _asbp_wfss_player_controller)
  (bind _returnvalue (`WizardFortressPlayerController.GetUIManager` _asbp_wfss_player_controller))
  (`UIManagerComponent.OpenInventoryTransferScreen` _returnvalue "/Game/UI/Screens/WBP_InvetoryTransferScreen.WBP_InvetoryTransferScreen_C" (`BaseCharacter.GetInventoryComponent` (`self.ChestOpener`)) (`self.Inventory`))
  (add `UIManagerComponent.OnLastScreenClosed` _returnvalue (delegate `HandleOnLastScreenClosed`))
  (bind (_direction _lidrotationx) (`Timeline|Timeline`)
    (:`Update`
      (`SceneComponent.K2_SetRelativeRotation` (`self.ChestLid`) (`KismetMathLibrary.MakeRotator` _lidrotationx) false false))
    (:`Finished`
      (`WizardFortressPlayerController.ChangeInputMapping` _asbp_wfss_player_controller "UI"))))

(event `self.InteractArea.OnComponentBeginOverlap`
  (params (OverlappedComponent :type "PrimitiveComponent Object Reference") (OtherActor :type "Actor Object Reference") (OtherComp :type "PrimitiveComponent Object Reference") (OtherBodyIndex :type Integer) (bFromSweep :type Boolean) (SweepResult :type "HitResult Structure (by ref)"))
  (if (`KismetSystemLibrary.DoesImplementInterface` OtherActor "/Script/WizardFortress.Interactor")
    (message `Interactor.AddInteractable` OtherActor self)))

(event `HandleOnLastScreenClosed`
  (bind (_direction _lidrotationx) (`Timeline|Timeline_0`)
    (:`Update`
      (`SceneComponent.K2_SetRelativeRotation` (`self.ChestLid`) (`KismetMathLibrary.MakeRotator` _lidrotationx) false false))))

(event `self.InteractArea.OnComponentEndOverlap`
  (params (OverlappedComponent :type "PrimitiveComponent Object Reference") (OtherActor :type "Actor Object Reference") (OtherComp :type "PrimitiveComponent Object Reference") (OtherBodyIndex :type Integer))
  (if (`KismetSystemLibrary.DoesImplementInterface` OtherActor "/Script/WizardFortress.Interactor")
    (message `Interactor.RemoveInteractable` OtherActor)))

(fn `GetAllItems`
  (returns (Items :type "Array of ItemData Object Reference"))
  (return))

(fn `GetItem`
  (params (RequestedItem :type "InventorySlot Structure"))
  (returns (Item :type "InventorySlot Structure"))
  (locals (ItemSlot :type "InventorySlot Structure"))
  (set `local.ItemSlot` RequestedItem))

(fn `ListItems`)

(fn `OpenAnimation`)

(fn `UserConstructionScript`)