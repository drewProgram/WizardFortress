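; BP_AICharTest is a test AI character that takes damage and can jump to a given destination.
; Any damage plays a hit montage and subtracts the amount through its AttributeSystem.
; JumptoDestination launches it on a suggested projectile arc aimed 250 units above the target, zeroing falling braking deceleration as a workaround for a jump bug.
; OnLanded restores that deceleration once the jump ends.
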(event `self.ReceiveAnyDamage`
  (params (Damage :type "Float (single-precision)") (DamageType :type "DamageType Object Reference") (InstigatedBy :type "Controller Object Reference") (DamageCauser :type "Actor Object Reference"))
  (`self.PlayAnimMontage` (`self.HitMontage`))
  (`AttributeSystem.RequestUpdateHealth` (`self.AttributeSystem`) (* Damage -1.0)))

(event `self.JumpToDestination`
  (params (Destination :type "Vector Structure"))
  (bind _outlaunchvelocity (`GameplayStatics.SuggestProjectileVelocity_CustomArc` (`self.K2_GetActorLocation`) (`KismetMathLibrary.MakeVector` (.x Destination) (.y Destination) (+ 250.0 (.z Destination)))))
  (`KismetSystemLibrary.PrintText` "Hello")
  ; Hack needed, otherwise jump will bug
  (set `CharacterMovementComponent.BrakingDecelerationFalling` 0.0 (`self.CharacterMovement`))
  (`self.LaunchCharacter` _outlaunchvelocity true true)
  (set `self.bIsJumping` true))

(event `self.OnLanded`
  (params (Hit :type "HitResult Structure (by ref)"))
  ; Enabling break deceleration again when jump ended
  (if (`self.bIsJumping`)
    (set `self.bIsJumping` false)
    (set `CharacterMovementComponent.BrakingDecelerationFalling` 1500.0 (`self.CharacterMovement`))))

(fn `UserConstructionScript`)